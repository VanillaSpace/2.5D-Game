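; Actor component that billboards its owner's Paper2D flipbook sprite toward the player camera.
; BeginPlay finds the flipbook and ticks only if it is valid.
; Each tick sets the sprite's world yaw to camera yaw plus RotationOffset, keeping pitch and roll zero.
; GetSpriteDirectionality returns a unit vector for the camera's bearing relative to owner facing, minus that offset, though nothing here calls it.
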(event EventBeginPlay
  (bind _output_get (Variables|Default|SetSprite (Actor|GetComponentbyClass (Components|GetOwner) "/Script/Paper2D.PaperFlipbookComponent")))
  (Components|Tick|SetComponentTickEnabled (Utilities|IsValid _output_get)))

(event EventTick
  (params (DeltaSeconds :type Float%20%28single-precision%29))
  (CallFunction|OrientSpritetoCamera))

(fn GetSpriteDirectionality
  (bind _returnvalue (Game|GetPlayerCameraManager 0))
  (bind _returnvalue_2 (Components|GetOwner))
  (bind _returnvalue_3 (Components|GetOwner))
  (bind _rotationoffset (Variables|Default|GetRotationOffset))
  (bind _returnvalue_4 (Camera|GetCameraLocation _returnvalue))
  (bind _returnvalue_5 (Transformation|GetActorLocation _returnvalue_3))
  (bind _returnvalue_6 (Transformation|GetActorRotation _returnvalue_2))
  (bind _returnvalue_7 (Math|Rotator|FindLookatRotation _returnvalue_5 _returnvalue_4))
  (bind _returnvalue_8 (Utilities|Operators|Subtract (.yaw _returnvalue_7) (.yaw _returnvalue_6) _rotationoffset))
  (bind _returnvalue_9 (Class|KismetMathLibrary|CreateVectorfromYawPitch _returnvalue_8 0.0 1.0))
  (return (Math|Vector|MakeVector (.x _returnvalue_9) (.y _returnvalue_9) 0.0)))

(fn OrientSpritetoCamera
  (bind _sprite (Variables|Default|GetSprite)
    (:then
      (Transformation|SetWorldRotation _sprite (Math|Rotator|MakeRotator 0.0 0.0 (+ (.yaw (Camera|GetCameraRotation (Game|GetPlayerCameraManager 0))) (Variables|Default|GetRotationOffset))) false false))
    (:else)))